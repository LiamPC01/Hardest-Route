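; Room actor that locks the player in with four doors until the room is finished.
; Box overlap tracks the player, raising the doors with a sound after a short delay on entry and lowering them on exit.
; DecrementEnemyCount finishes the room whenever the count remains zero or above, not only at zero; H also finishes it while the player is inside.
; Tick keeps doors lowered in rooms flagged empty.
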(event OnComponentBeginOverlap(Box)
  (params (OverlappedComponent :type Primitive%20Component%20Object%20Reference) (OtherActor :type Actor%20Object%20Reference) (OtherComp :type Primitive%20Component%20Object%20Reference) (OtherBodyIndex :type Integer) (bFromSweep :type Boolean) (SweepResult :type Hit%20Result%20Structure%20%28by%20ref%29))
  (bind _asbp_top_down_character (Utilities|Casting|CastToBP_TopDownCharacter OtherActor))
  (Utilities|IsValid _asbp_top_down_character
    (:Is%20Valid
      (Variables|Default|SetplayerInside true)
      (Utilities|FlowControl|Delay 0.7)
      (CallFunction|UpdateDoors))))

(event OnComponentEndOverlap(Box)
  (params (OverlappedComponent :type Primitive%20Component%20Object%20Reference) (OtherActor :type Actor%20Object%20Reference) (OtherComp :type Primitive%20Component%20Object%20Reference) (OtherBodyIndex :type Integer))
  (bind _asbp_top_down_character (Utilities|Casting|CastToBP_TopDownCharacter OtherActor))
  (Utilities|IsValid _asbp_top_down_character
    (:Is%20Valid
      (Variables|Default|SetplayerInside false)
      (CallFunction|UpdateDoors))
    (:Is%20Not%20Valid
      (bind _asenemy_bp (Utilities|Casting|CastToEnemy_BP OtherActor))
      (Utilities|IsValid _asenemy_bp
        (:Is%20Valid
          (bind _output_get (Variables|Default|SetEnemyCount (+ 1 (Variables|Default|GetEnemyCount))))
          (Development|PrintString (Utilities|String|ToString(Integer) _output_get)))))))

(event Custom|UpdateDoors
  (bind _door_south (Variables|Default|GetDoor_South))
  (bind _door_west (Variables|Default|GetDoor_West))
  (bind _door_south_2 (Variables|Default|GetDoor_South))
  (bind _door_west_2 (Variables|Default|GetDoor_West))
  (bind _door_north (Variables|Default|GetDoor_North))
  (bind _door_east (Variables|Default|GetDoor_East))
  (bind _returnvalue (Transformation|GetRelativeTransform _door_west))
  (bind _returnvalue_2 (Transformation|GetRelativeTransform _door_north))
  (bind _returnvalue_3 (Transformation|GetRelativeTransform _door_north))
  (bind _returnvalue_4 (Transformation|GetRelativeTransform _door_east))
  (bind _returnvalue_5 (Transformation|GetRelativeTransform _door_south_2))
  (bind _returnvalue_6 (Transformation|GetRelativeTransform _door_east))
  (bind _returnvalue_7 (Transformation|GetRelativeTransform _door_west_2))
  (bind _returnvalue_8 (Transformation|GetRelativeTransform _door_south))
  (if (Variables|Default|GetplayerInside)
    (CallFunction|DoorSoundEffect)
    (Transformation|SetRelativeLocation _door_north (Math|Vector|MakeVector (.x (.location _returnvalue_3)) (.y (.location _returnvalue_3)) 0.0) false false)
    (Transformation|SetRelativeLocation _door_east (Math|Vector|MakeVector (.x (.location _returnvalue_6)) (.y (.location _returnvalue_6)) 0.0) false false)
    (Transformation|SetRelativeLocation _door_south (Math|Vector|MakeVector (.x (.location _returnvalue_8)) (.y (.location _returnvalue_8)) 0.0) false false)
    (Transformation|SetRelativeLocation _door_west (Math|Vector|MakeVector (.x (.location _returnvalue)) (.y (.location _returnvalue)) 0.0) false false)
    (else
      (Transformation|SetRelativeLocation _door_north (Math|Vector|MakeVector (.x (.location _returnvalue_2)) (.y (.location _returnvalue_2)) -5e+02) false false)
      (Transformation|SetRelativeLocation _door_east (Math|Vector|MakeVector (.x (.location _returnvalue_4)) (.y (.location _returnvalue_4)) -5e+02) false false)
      (Transformation|SetRelativeLocation _door_south_2 (Math|Vector|MakeVector (.x (.location _returnvalue_5)) (.y (.location _returnvalue_5)) -5e+02) false false)
      (Transformation|SetRelativeLocation _door_west_2 (Math|Vector|MakeVector (.x (.location _returnvalue_7)) (.y (.location _returnvalue_7)) -5e+02) false false))))

(event Custom|FinishedRoom
  (bind _door_south (Variables|Default|GetDoor_South))
  (bind _door_west (Variables|Default|GetDoor_West))
  (bind _door_north (Variables|Default|GetDoor_North))
  (bind _door_east (Variables|Default|GetDoor_East))
  (bind _returnvalue (Transformation|GetRelativeTransform _door_north))
  (bind _returnvalue_2 (Transformation|GetRelativeTransform _door_east))
  (bind _returnvalue_3 (Transformation|GetRelativeTransform _door_south))
  (bind _returnvalue_4 (Transformation|GetRelativeTransform _door_west))
  (if (Variables|Default|GetplayerFinishedRoom)
    (Transformation|SetRelativeLocation _door_north (Math|Vector|MakeVector (.x (.location _returnvalue)) (.y (.location _returnvalue)) -5e+02) false false)
    (Transformation|SetRelativeLocation _door_east (Math|Vector|MakeVector (.x (.location _returnvalue_2)) (.y (.location _returnvalue_2)) -5e+02) false false)
    (Transformation|SetRelativeLocation _door_south (Math|Vector|MakeVector (.x (.location _returnvalue_3)) (.y (.location _returnvalue_3)) -5e+02) false false)
    (Transformation|SetRelativeLocation _door_west (Math|Vector|MakeVector (.x (.location _returnvalue_4)) (.y (.location _returnvalue_4)) -5e+02) false false)))

(event Custom|DoorSoundEffect
  (Audio|PlaySound2D "/Game/Oli_BPs/Audio/Door.Door" 1.0 1.0 0.0 0 0))

(event EventBeginPlay
  (Variables|Default|SetplayerInside false)
  (CallFunction|UpdateDoors))

(event Collision|EventActorBeginOverlap
  (params (OtherActor :type Actor%20Object%20Reference)))

(event EventTick
  (params (DeltaSeconds :type Float%20%28single-precision%29))
  (bind _door_west (Variables|Default|GetDoor_West))
  (bind _door_north (Variables|Default|GetDoor_North))
  (bind _door_east (Variables|Default|GetDoor_East))
  (bind _door_south (Variables|Default|GetDoor_South))
  (bind _returnvalue (Transformation|GetRelativeTransform _door_west))
  (bind _returnvalue_2 (Transformation|GetRelativeTransform _door_north))
  (bind _returnvalue_3 (Transformation|GetRelativeTransform _door_east))
  (bind _returnvalue_4 (Transformation|GetRelativeTransform _door_south))
  (if (Variables|Default|GetIsEmpty)
    (Transformation|SetRelativeLocation _door_north (Math|Vector|MakeVector (.x (.location _returnvalue_2)) (.y (.location _returnvalue_2)) -5e+02) false false)
    (Transformation|SetRelativeLocation _door_east (Math|Vector|MakeVector (.x (.location _returnvalue_3)) (.y (.location _returnvalue_3)) -5e+02) false false)
    (Transformation|SetRelativeLocation _door_south (Math|Vector|MakeVector (.x (.location _returnvalue_4)) (.y (.location _returnvalue_4)) -5e+02) false false)
    (Transformation|SetRelativeLocation _door_west (Math|Vector|MakeVector (.x (.location _returnvalue)) (.y (.location _returnvalue)) -5e+02) false false)))

(event Input|KeyboardEvents|H
  (params (Key :type Key%20Structure :default "None"))
  (:Pressed
    (if (Variables|Default|GetplayerInside)
      (Variables|Default|SetplayerFinishedRoom true)
      (CallFunction|FinishedRoom))))

(fn ConstructionScript)

(fn DecrementEnemyCount
  (bind _result (Math|Integer|DecrementInt (Variables|Default|GetEnemyCount))
    (:%20%20
      (bind _output_get (Variables|Default|SetEnemyCount _result))
      (Development|PrintString (Utilities|String|ToString(Integer) _output_get))
      (if (<= 0 (Variables|Default|GetEnemyCount))
        (Variables|Default|SetplayerFinishedRoom true)
        (Variables|Default|SetplayerInside false)
        (CallFunction|FinishedRoom)))))

(fn IncrementEnemyCount
  (bind _result (Math|Integer|IncrementInt (Variables|Default|GetEnemyCount))
    (:%20%20
      (Variables|Default|SetEnemyCount _result))))
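; Enemy character Blueprint that reacts when the top-down player character enters its AttackBox.
; While it has Stamina, each such overlap calls IncreaseScore on the player and then SpendStamina.
; SpendStamina deducts a fixed amount, prints debug text and disables the enemy's movement once Stamina runs out, with no recovery in this graph.
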(event OnComponentBeginOverlap(AttackBox)
  (params (OverlappedComponent :type Primitive%20Component%20Object%20Reference) (OtherActor :type Actor%20Object%20Reference) (OtherComp :type Primitive%20Component%20Object%20Reference) (OtherBodyIndex :type Integer) (bFromSweep :type Boolean) (SweepResult :type Hit%20Result%20Structure%20%28by%20ref%29))
  (if (> (Variables|Default|GetStamina) 0)
    (bind _asbp_top_down_character (Utilities|Casting|CastToBP_TopDownCharacter OtherActor))
    (Default|IncreaseScore _asbp_top_down_character)
    (CallFunction|SpendStamina)))

(event EventBeginPlay)

(event Collision|EventActorBeginOverlap
  (params (OtherActor :type Actor%20Object%20Reference)))

(event EventTick
  (params (DeltaSeconds :type Float%20%28single-precision%29)))

(fn ConstructionScript)

(fn SpendStamina
  (if (> (Variables|Default|GetStamina) 0)
    (bind _output_get (Variables|Default|SetStamina (- (Variables|Default|GetStamina) 25)))
    (Development|PrintString (Utilities|String|ToString(Integer) _output_get))
    (if (not (> (Variables|Default|GetStamina) 0))
      (Development|PrintString "disable character niovenebt]")
      (Pawn|Components|CharacterMovement|DisableMovement (Variables|Character|GetCharacterMovement)))))
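; Enemy healer character that reacts when a BP_TopDownCharacter enters or leaves its HealBox trigger; no healing logic is implemented here.
; On overlap it sets its own movement mode to None, spends one point of HealerStamina and calls DecreaseScore on that character.
; When the character leaves, it returns to Walking.
; SpendStamina prints the remaining value and has no lower limit or regeneration.
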(event OnComponentBeginOverlap(HealBox)
  (params (OverlappedComponent :type Primitive%20Component%20Object%20Reference) (OtherActor :type Actor%20Object%20Reference) (OtherComp :type Primitive%20Component%20Object%20Reference) (OtherBodyIndex :type Integer) (bFromSweep :type Boolean) (SweepResult :type Hit%20Result%20Structure%20%28by%20ref%29))
  (bind _asbp_top_down_character (Utilities|Casting|CastToBP_TopDownCharacter OtherActor))
  (Pawn|Components|CharacterMovement|SetMovementMode (Variables|Character|GetCharacterMovement) "MOVE_None" 0)
  (CallFunction|SpendStamina)
  (Default|DecreaseScore _asbp_top_down_character))

(event OnComponentEndOverlap(HealBox)
  (params (OverlappedComponent :type Primitive%20Component%20Object%20Reference) (OtherActor :type Actor%20Object%20Reference) (OtherComp :type Primitive%20Component%20Object%20Reference) (OtherBodyIndex :type Integer))
  (Utilities|Casting|CastToBP_TopDownCharacter OtherActor)
  (Pawn|Components|CharacterMovement|SetMovementMode (Variables|Character|GetCharacterMovement) "MOVE_Walking" 0))

(event EventBeginPlay)

(event Collision|EventActorBeginOverlap
  (params (OtherActor :type Actor%20Object%20Reference)))

(event EventTick
  (params (DeltaSeconds :type Float%20%28single-precision%29)))

(fn ConstructionScript)

(fn SpendStamina
  (bind _output_get (Variables|Default|SetHealerStamina (- (Variables|Default|GetHealerStamina) 1.0)))
  (Development|PrintString (Utilities|String|ToString(Float) _output_get)))
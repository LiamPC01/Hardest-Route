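; Enemy character that attacks a player inside its AttackBox and passes out once its stamina is exhausted.
; Tick drives the attack, raising player score, spending stamina, timing animation and headbutt sound with Delays, and clearing then restoring the target as a cooldown.
; Capsule overlap registers it in a Room_BP's enemy count.
; At zero stamina it disables movement, sets the passed-out animation state and decrements that count.
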(event OnComponentBeginOverlap(AttackBox)
  (params (OverlappedComponent :type Primitive%20Component%20Object%20Reference) (OtherActor :type Actor%20Object%20Reference) (OtherComp :type Primitive%20Component%20Object%20Reference) (OtherBodyIndex :type Integer) (bFromSweep :type Boolean) (SweepResult :type Hit%20Result%20Structure%20%28by%20ref%29))
  (bind _asbp_top_down_character (Utilities|Casting|CastToBP_TopDownCharacter OtherActor))
  (Variables|Default|SetPlayerTarget _asbp_top_down_character))

(event OnComponentEndOverlap(AttackBox)
  (params (OverlappedComponent :type Primitive%20Component%20Object%20Reference) (OtherActor :type Actor%20Object%20Reference) (OtherComp :type Primitive%20Component%20Object%20Reference) (OtherBodyIndex :type Integer))
  (Utilities|Casting|CastToBP_TopDownCharacter OtherActor)
  (Variables|Default|SetPlayerTarget 0))

(event OnComponentBeginOverlap(CapsuleComponent)
  (params (OverlappedComponent :type Primitive%20Component%20Object%20Reference) (OtherActor :type Actor%20Object%20Reference) (OtherComp :type Primitive%20Component%20Object%20Reference) (OtherBodyIndex :type Integer) (bFromSweep :type Boolean) (SweepResult :type Hit%20Result%20Structure%20%28by%20ref%29))
  (bind _asroom_bp (Utilities|Casting|CastToRoom_BP OtherActor))
  (Utilities|IsValid _asroom_bp
    (:Is%20Valid
      (bind _output_get (Variables|Default|SetRoom _asroom_bp))
      (Default|IncrementEnemyCount _output_get)
      (Development|PrintString (Utilities|GetDisplayName _output_get)))))

(event EventBeginPlay)

(event Collision|EventActorBeginOverlap
  (params (OtherActor :type Actor%20Object%20Reference)))

(event EventTick
  (params (DeltaSeconds :type Float%20%28single-precision%29))
  (bind _bispassedout (CallFunction|CheckStamina))
  (if (and (!= _bispassedout true) (Utilities|IsValid (Variables|Default|GetPlayerTarget)))
    (Variables|Default|SetPlayerTarget 0)
    (Default|IncreaseScore (stale OnComponentBeginOverlap(AttackBox) _asbp_top_down_character))
    (CallFunction|CheckStamina)
    (CallFunction|SpendStamina)
    (bind _newparam (CallFunction|TriggerAttackAnim))
    (Utilities|FlowControl|Delay 0.7)
    (Default|HeadbuttSound (stale OnComponentBeginOverlap(AttackBox) _asbp_top_down_character))
    (Utilities|FlowControl|Delay 1.0)
    (Variables|/Game/Liam-New/Liam_Enemy/EnemyModel/NEWEnemyAnim_BP.NEWEnemyAnim_BP_C|SetBIsAttacking _newparam false)
    (CallFunction|CheckStamina)
    (Utilities|FlowControl|Delay 2.0)
    (Variables|Default|SetPlayerTarget (stale OnComponentBeginOverlap(AttackBox) _asbp_top_down_character))))

(fn ConstructionScript)

(fn SpendStamina
  (if (> (Variables|Default|GetStamina) 0)
    (bind _output_get (Variables|Default|SetStamina (- (Variables|Default|GetStamina) 25)))
    (Development|PrintString (Utilities|String|ToString(Integer) _output_get))
    (if (not (> (Variables|Default|GetStamina) 0))
      (Development|PrintString "disable character niovenebt]")
      (Pawn|Components|CharacterMovement|DisableMovement (Variables|Character|GetCharacterMovement)))))

(fn CheckStamina
  (if (not (> (Variables|Default|GetStamina) 0))
    (bind _asnewenemy_anim_bp (Utilities|Casting|CastToNEWEnemyAnim_BP (Components|SkeletalMesh|GetAnimInstance (Variables|Default|GetSkeletalMesh))))
    (Variables|/Game/Liam-New/Liam_Enemy/EnemyModel/NEWEnemyAnim_BP.NEWEnemyAnim_BP_C|SetBIsAttacking _asnewenemy_anim_bp false)
    (Variables|/Game/Liam-New/Liam_Enemy/EnemyModel/NEWEnemyAnim_BP.NEWEnemyAnim_BP_C|SetBIsPassedOut _asnewenemy_anim_bp true)
    (if (>= (Variables|/Game/Oli_BPs/Room_BP.Room_BP_C|GetEnemyCount (Variables|Default|GetRoom)) 0)
      (Default|DecrementEnemyCount (Variables|Default|GetRoom))
      (return true))))

(fn TriggerAttackAnim
  (Development|PrintString "trigger anim")
  (bind _asnewenemy_anim_bp (Utilities|Casting|CastToNEWEnemyAnim_BP (Components|SkeletalMesh|GetAnimInstance (Variables|Default|GetSkeletalMesh)))
    (:then
      (Variables|/Game/Liam-New/Liam_Enemy/EnemyModel/NEWEnemyAnim_BP.NEWEnemyAnim_BP_C|SetBIsAttacking _asnewenemy_anim_bp true))
    (:CastFailed
      _))
  (return _asnewenemy_anim_bp))

(fn UpdateRoom)